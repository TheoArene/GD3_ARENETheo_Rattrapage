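; BP_Balle is a physics-driven ball actor that launches along the X axis when play begins and gets faster each time it bounces.
; BeginPlay gives the Balle component an initial velocity-change impulse.
; Every Hit event increments BalleSpeed, then clamps the current physics velocity to exactly that magnitude, preserving direction while enforcing the new speed.
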(event `self.ReceiveBeginPlay`
  (`PrimitiveComponent.AddImpulse` (`self.Balle`) (1200.0 0.0 0.0) "None" true))

(event `self.ReceiveHit`
  (params (MyComp :type "PrimitiveComponent Object Reference") (Other :type "Actor Object Reference") (OtherComp :type "PrimitiveComponent Object Reference") (bSelfMoved :type Boolean) (HitLocation :type "Vector Structure") (HitNormal :type "Vector Structure") (NormalImpulse :type "Vector Structure") (Hit :type "HitResult Structure (by ref)"))
  (bind _ballespeed (`self.BalleSpeed`))
  (set `self.BalleSpeed` (+ (`self.BalleSpeed`) 4.0))
  (bind _returnvalue (`PrimitiveComponent.GetPhysicsLinearVelocity` (`self.Balle`) "None"))
  (`PrimitiveComponent.SetPhysicsLinearVelocity` (`self.Balle`) (`KismetMathLibrary.ClampVectorSize` _returnvalue _ballespeed _ballespeed) false "None"))

(fn `UserConstructionScript`)