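; Player-controlled paddle (raquette) for a brick-breaker game.
; On BeginPlay it adds the IMC_CasseBrique Enhanced Input mapping context to its player controller, then creates the WBP_Score widget, stores it and shows it on screen.
; IA_Move input slides the paddle along its local Z axis, scaled by RaquetteSpeed without delta time, using a swept offset so blocking collision stops it.
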(event `self.ReceiveBeginPlay`
  (bind _asplayer_controller (cast `PlayerController` (`self.GetController`)))
  (bind _returnvalue (pcsubsystem `EnhancedInputLocalPlayerSubsystem` _asplayer_controller))
  (`/Engine/EditorBlueprintResources/StandardMacros.IsValid` _returnvalue
    (:`Is Valid`
      (`EnhancedInputSubsystemInterface.AddMappingContext` _returnvalue "/Game/Input/IMC_CasseBrique.IMC_CasseBrique" 0 (struct))
      (bind _returnvalue_2 (`|CreateWidget` "/Game/Widget/WBP_Score.WBP_Score_C"))
      (bind _output_get (set `self.ScoreJoueur` _returnvalue_2))
      (`UserWidget.AddToViewport` _output_get 0))))

(event `EnhancedInput|/Game/Input/IA_Move`
  (params (ActionValue :type "Float (double-precision)") (ElapsedSeconds :type "Float (double-precision)") (TriggeredSeconds :type "Float (double-precision)") (InputAction :type "InputAction Object Reference" :default "/Game/Input/IA_Move.IA_Move"))
  ;[1 1 1] Fait bouger la raquette par rapport a IA_Move
  (:`Triggered`
    (`SceneComponent.K2_AddLocalOffset` (`self.Raquette`) (`KismetMathLibrary.MakeVector` 0.0 0.0 (* ActionValue (`self.RaquetteSpeed`))) true false)))

(fn `UserConstructionScript`)