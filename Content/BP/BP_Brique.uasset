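; Breakout-style brick that takes hits from BP_Balle until its BriqueStrenght runs out.
; UpdateBriqueColor maps the remaining strength to a green, yellow or red glow material, both at construction and after each non-fatal hit with a sound.
; The fatal hit spawns an explosion and sound, then destroys the brick.
; If no bricks remain, it shows WBP_Win, pauses the game and displays the mouse cursor.
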(event `self.ReceiveHit`
  (params (MyComp :type "PrimitiveComponent Object Reference") (Other :type "Actor Object Reference") (OtherComp :type "PrimitiveComponent Object Reference") (bSelfMoved :type Boolean) (HitLocation :type "Vector Structure") (HitNormal :type "Vector Structure") (NormalImpulse :type "Vector Structure") (Hit :type "HitResult Structure (by ref)"))
  ;[1 1 1] Défini que lorsque la balle touche la brique, en fonction de la couleur selectionné, la balle va devoir rebondir un certain nbr de fois dessus avant de détruire la brique
  (cast `/Game/BP/BP_Balle` Other)
  (bind _result (`/Engine/EditorBlueprintResources/StandardMacros.DecrementInt` (`self.BriqueStrenght`))
    (:`  `
      (if (== _result 0)
        (`GameplayStatics.SpawnEmitterAtLocation` "/Game/StarterContent/Particles/P_Explosion.P_Explosion" (`self.K2_GetActorLocation`))
        (`GameplayStatics.PlaySoundAtLocation` "/Game/Sound/Damage.Damage" (`self.K2_GetActorLocation`) (struct) 1.0 1.0 0.0 null null null null)
        (`self.K2_DestroyActor`)
        (bind _outactors (`GameplayStatics.GetAllActorsOfClass` "BP_Brique_C"))
        (if (== (`KismetArrayLibrary.Array_Length` _outactors) 0)
          (bind _returnvalue (`|CreateWidget` "/Game/Widget/WBP_Win.WBP_Win_C"))
          (`UserWidget.AddToViewport` _returnvalue 0)
          (`GameplayStatics.SetGamePaused` true)
          (set `PlayerController.bShowMouseCursor` true (`GameplayStatics.GetPlayerController` 0)))
        (else
          (`GameplayStatics.PlaySoundAtLocation` "/Game/Sound/Destruction.Destruction" (`self.K2_GetActorLocation`) (struct) 1.0 1.0 0.0 null null null null)
          (`self.UpdateBriqueColor`))))))

(fn `UpdateBriqueColor`
  (bind _brique (`self.Brique`))
  ;[1 1 1] permet de définir la couleur ainsi que la durée de vie d'une brique
  (switch `int` (`self.BriqueStrenght`)
    (:`1`
      (`PrimitiveComponent.SetMaterial` _brique 0 "/Game/Materials/MI_GlowGreen.MI_GlowGreen"))
    (:`2`
      (`PrimitiveComponent.SetMaterial` _brique 0 "/Game/Materials/MI_GlowYellow.MI_GlowYellow"))
    (:`3`
      (`PrimitiveComponent.SetMaterial` _brique 0 "/Game/Materials/MI_GlowRed.MI_GlowRed"))))

(fn `UserConstructionScript`
  (`self.UpdateBriqueColor`))