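; Brick for a brick-breaker style game that loses one point of BriqueStrenght2 each time a BP_Balle hits it.
; At zero it spawns an explosion and destroys itself; otherwise it calls a colour update, also run by the construction script.
; That update maps levels to glow materials on BalleXXXXXX, but its switch reads a constant 0 instead of the strength, so no material is applied.
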(event `self.ReceiveHit`
  (params (MyComp :type "PrimitiveComponent Object Reference") (Other :type "Actor Object Reference") (OtherComp :type "PrimitiveComponent Object Reference") (bSelfMoved :type Boolean) (HitLocation :type "Vector Structure") (HitNormal :type "Vector Structure") (NormalImpulse :type "Vector Structure") (Hit :type "HitResult Structure (by ref)"))
  (cast `/Game/BP/BP_Balle` Other)
  (bind _result (`/Engine/EditorBlueprintResources/StandardMacros.DecrementInt` (`self.BriqueStrenght2`))
    (:`  `
      (if (== _result 0)
        (`GameplayStatics.SpawnEmitterAtLocation` "/Game/StarterContent/Particles/P_Explosion.P_Explosion" (`self.K2_GetActorLocation`))
        (`self.K2_DestroyActor`)
        (else
          (`self.Definir couleur brique balleXXXXXX`))))))

(fn `Definir couleur brique balleXXXXXX`
  (bind _ballexxxxxx (`self.BalleXXXXXX`))
  (switch `int` 0
    (:`1`
      (`PrimitiveComponent.SetMaterial` _ballexxxxxx 0 "/Game/Materials/MI_GlowGreen.MI_GlowGreen"))
    (:`2`
      (`PrimitiveComponent.SetMaterial` _ballexxxxxx 0 "/Game/Materials/MI_GlowYellow.MI_GlowYellow"))
    (:`3`
      (`PrimitiveComponent.SetMaterial` _ballexxxxxx 0 "/Game/Materials/MI_GlowRed.MI_GlowRed"))
    (:`4`
      (`PrimitiveComponent.SetMaterial` _ballexxxxxx 0 "/Game/Materials/MI_GlowRed.MI_GlowRed"))))

(fn `UserConstructionScript`
  (`self.Definir couleur brique balleXXXXXX`))